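; BP_Camera is a player view camera actor with mouse panning, zoom and focus on a location.
; While right mouse is held, a looping 0.01-second timer applies swept offsets proportional to cursor distance from the press point, clamped to a maximum.
; The mouse wheel adjusts spring arm length within limits.
; FocusOn plays a timeline that lerps the root between target and current location, and StopFocus halts it.
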(event Custom|TickEvent
  (bind _returnvalue (Utilities|Time|GetWorldDeltaSeconds))
  (bind _returnvalue_2 (Game|GetPlayerController 0))
  (bind _initmousepos (Variables|Default|GetInitMousePos))
  (bind _panningspeed (Variables|Default|GetPanningSpeed))
  (bind _maxpanningspeed (Variables|Default|GetMaxPanningSpeed))
  (bind _returnvalue_3 (- 0.0 _maxpanningspeed))
  (bind (_locationx _locationy) (Game|Player|GetMousePosition _returnvalue_2))
  (if (Variables|Default|GetisPanning)
    (Transformation|AddActorWorldOffset (Math|Vector|MakeVector (Math|Float|Clamp(Float) (* (- _locationy (.y _initmousepos)) _panningspeed _returnvalue) _returnvalue_3 _maxpanningspeed) (Math|Float|Clamp(Float) (* (- (.x _initmousepos) _locationx) _panningspeed _returnvalue) _returnvalue_3 _maxpanningspeed) 0.0) true)))

(event Custom|FocusOn
  (params (TargetLoc :type Vector))
  (bind _defaultsceneroot (Variables|Default|GetDefaultSceneRoot))
  (bind _returnvalue (Transformation|GetWorldLocation _defaultsceneroot))
  (bind _newtrack_0 (Timeline|FocusLerp PlayFromStart)
    (:Update
      (Transformation|SetWorldLocation (Variables|Default|GetDefaultSceneRoot) (Math|Vector|Lerp(Vector) (Math|Vector|MakeVector (.x TargetLoc) (.y TargetLoc) 0.0) (Math|Vector|MakeVector (.x _returnvalue) (.y _returnvalue) 0.0) _newtrack_0) true false))))

(event Custom|StopFocus
  (bind _defaultsceneroot (Variables|Default|GetDefaultSceneRoot))
  (bind _returnvalue (Transformation|GetWorldLocation _defaultsceneroot))
  (bind _newtrack_0 (Timeline|FocusLerp Stop)
    (:Update
      (Transformation|SetWorldLocation (Variables|Default|GetDefaultSceneRoot) (Math|Vector|Lerp(Vector) (Math|Vector|MakeVector (.x (stale Custom|FocusOn TargetLoc)) (.y (stale Custom|FocusOn TargetLoc)) 0.0) (Math|Vector|MakeVector (.x _returnvalue) (.y _returnvalue) 0.0) _newtrack_0) true false))))

(event EventBeginPlay
  (Game|Player|SetViewTargetwithBlend (Game|GetPlayerController 0) self 0.0 "VTBlend_Linear" 0.0 false)
  (Utilities|Time|SetTimerbyEvent (delegate Custom|TickEvent) 0.01 true))

(event Collision|EventActorBeginOverlap
  (params (OtherActor :type Actor%20Object%20Reference)))

(event EventTick
  (params (DeltaSeconds :type Float%20%28single-precision%29)))

(event Input|MouseEvents|MouseWheelAxis
  (params (AxisValue :type Float%20%28single-precision%29))
  (Variables|/Script/Engine.SpringArmComponent|SetTargetArmLength (Variables|Default|GetSpringArm) (Math|Float|Clamp(Float) (+ (Variables|/Script/Engine.SpringArmComponent|GetTargetArmLength (Variables|Default|GetSpringArm)) (* AxisValue -1e+02)) 5e+02 2e+03)))

(event Input|MouseEvents|RightMouseButton
  (params (Key :type Key%20Structure))
  (bind _returnvalue (Game|GetPlayerController 0))
  (bind (_locationx _locationy) (Game|Player|GetMousePosition _returnvalue))
  (:Pressed
    (Variables|Default|SetisPanning true)
    (Variables|Default|SetInitMousePos (Math|Vector2D|MakeVector2D _locationx _locationy)))
  (:Released
    (Variables|Default|SetisPanning false)))

(fn ConstructionScript)