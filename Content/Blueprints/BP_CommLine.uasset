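; BP_CommLine is a construction-time line actor that draws a spline mesh between its StartPoint and EndPoint components.
; The construction script pins the spline to both points, samples it at even intervals set by NumberOfBetweenPoints, then rebuilds it from those locations and tangents.
; Each segment gets a Z-forward spline mesh component, manually attached and placed using world-space positions and tangents.
; The event graph has no active logic.
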(event EventBeginPlay)

(event Collision|EventActorBeginOverlap
  (params (OtherActor :type Actor%20Object%20Reference)))

(event EventTick
  (params (DeltaSeconds :type Float%20%28single-precision%29)))

(fn ConstructionScript
  (bind _spline (Variables|Default|GetSpline))
  (bind _spline_2 (Variables|Default|GetSpline))
  (bind _spline_3 (Variables|Default|GetSpline))
  (bind _returnvalue (Spline|GetNumberOfSplinePoints _spline))
  (bind _returnvalue_2 (- _returnvalue 1))
  (Spline|SetLocationatSplinePoint (Variables|Default|GetSpline) 0 (Transformation|GetWorldLocation (Variables|Default|GetStartPoint)) "World" true)
  (Spline|SetLocationatSplinePoint (Variables|Default|GetSpline) 1 (Transformation|GetWorldLocation (Variables|Default|GetEndPoint)) "World" true)
  (Utilities|FlowControl|Sequence
    (:then_0
      (LocalVariables|SetDistBetweenPoint (/ (Spline|GetSplineLength (Variables|Default|GetSpline)) (Math|Conversions|ToFloat(Integer) (+ (LocalVariables|GetNumberOfBetweenPoints) 1))))
      (for _index (range 0 (+ (LocalVariables|GetNumberOfBetweenPoints) 1))
        (Utilities|Array|Add (LocalVariables|GetPointLocation) (Spline|GetLocationatDistanceAlongSpline _spline_3 (* _index (LocalVariables|GetDistBetweenPoint)) "Local"))
        (Utilities|Array|Add (LocalVariables|GetPointTangent) (Spline|GetTangentatDistanceAlongSpline _spline_3 (* _index (LocalVariables|GetDistBetweenPoint)) "Local")))
      (Spline|ClearSplinePoints (Variables|Default|GetSpline) true))
    (:then_1
      (for _index_2 (range 0 (+ (LocalVariables|GetNumberOfBetweenPoints) 1))
        (Spline|AddSplinePoint (Variables|Default|GetSpline) (Utilities|Array|Get(acopy) (LocalVariables|GetPointLocation) _index_2) "Local" true)
        (Spline|SetTangentatSplinePoint (Variables|Default|GetSpline) _index_2 (Utilities|Array|Get(acopy) (LocalVariables|GetPointTangent) _index_2) "Local" true)))
    (:then_2
      (for _index_3 (range 0 _returnvalue_2)
        (if (!= _index_3 _returnvalue_2)
          (bind _returnvalue_3 (AddComponent|AddSplineMeshComponent true))
          (SplineMesh|SetForwardAxis _returnvalue_3 "Z" true)
          (SplineMesh|SetStartandEnd _returnvalue_3 (Spline|GetLocationatSplinePoint _spline_2 _index_3 "World") (Spline|GetTangentatSplinePoint _spline_2 _index_3 "World") (Spline|GetLocationatSplinePoint _spline_2 (+ _index_3 1) "World") (Spline|GetTangentatSplinePoint _spline_2 (+ _index_3 1) "World") true :!class /Script/Engine.SplineMeshComponent))))))