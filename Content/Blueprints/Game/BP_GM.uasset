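; BP_GM drives the game's passive gold economy and HUD, and holds an unfinished house-spawning function.
; On BeginPlay it caches BP_GI, starts a looping one-second timer that adds GoldPerSecond to its Gold, and shows BP_HUD.
; SpawnNewHouse picks a randomized offset from a start house and sphere-traces there with debug drawing, but ignores the result.
; Its nodes for spawning BP_House and a connecting BP_CommLine are disconnected, so never run.
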(event Custom|GoldIncrement
  (bind _giref (Variables|Default|GetGIRef))
  (Variables|/Game/Blueprints/Game/BP_GI.BP_GI_C|SetGold (Variables|Default|GetGIRef) (+ (Variables|/Game/Blueprints/Game/BP_GI.BP_GI_C|GetGold _giref) (Variables|/Game/Blueprints/Game/BP_GI.BP_GI_C|GetGoldPerSecond _giref))))

(event EventBeginPlay
  (bind _asbp_gi (Utilities|Casting|CastToBP_GI (Game|GetGameInstance)))
  (Variables|Default|SetGIRef _asbp_gi)
  (Utilities|Time|SetTimerbyEvent (delegate Custom|GoldIncrement) 1.0 true)
  (bind _returnvalue (UserInterface|CreateWidget "/Game/UI/BP_HUD.BP_HUD_C"))
  (bind _output_get (Variables|Default|SetHUDRef _returnvalue))
  (UserInterface|Viewport|AddtoViewport _output_get 0))

(event EventTick
  (params (DeltaSeconds :type Float%20%28single-precision%29)))

(fn ConstructionScript)

(fn SpawnNewHouse
  (params (StartHouse :type BP%20House%20Object%20Reference) (SpawnRadiusMin :type Float%20%28single-precision%29) (SpawnRadiusMax :type Float%20%28single-precision%29))
  (bind _returnvalue (Math|Random|RandomFloatinRange SpawnRadiusMin SpawnRadiusMax))
  (bind _returnvalue_2 (Math|Random|RandomFloatinRange 0.0 359.0))
  (bind _output_get (LocalVariables|SetStart StartHouse))
  (LocalVariables|SetStartLoc (Math|Vector|MakeVector (.x (Transformation|GetActorLocation _output_get)) (.y (Transformation|GetActorLocation _output_get)) (.z (Transformation|GetActorLocation _output_get))))
  (LocalVariables|SetEndLoc (Math|Vector|MakeVector (+ (.x (Transformation|GetActorLocation _output_get)) (* (Math|Trig|Cos(Degrees) _returnvalue_2) _returnvalue)) (+ (.y (Transformation|GetActorLocation _output_get)) (* (Math|Trig|Sin(Degrees) _returnvalue_2) _returnvalue)) (.z (Transformation|GetActorLocation _output_get))))
  (Utilities|FlowControl|ForLoopwithBreak 0 0
    (:LoopBody
      (bind _outhit (Collision|SphereTraceByChannel (LocalVariables|GetEndLoc) (LocalVariables|GetEndLoc) 1e+02 "TraceTypeQuery1" false 0 "ForDuration"))
      (if true
        _))))