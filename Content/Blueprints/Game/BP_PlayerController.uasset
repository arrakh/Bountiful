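; Player controller that handles click selection of world actors and debug hotkeys, caching the BP_Camera and BP_GM references on BeginPlay.
; Left click traces under the cursor, and a BPI_Interactables hit gets camera focus, becomes the current actor and receives a click message.
; Space asks the game mode to spawn a new house around the selected BP_House.
; Keys 1 to 4 send numbered debug messages to the selection.
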(event EventBeginPlay
  (bind _outactors (Actor|GetAllActorsOfClass "/Game/Blueprints/BP_Camera.BP_Camera_C"))
  (Variables|Default|SetCamRef (Utilities|Array|Get(acopy) _outactors))
  (bind _asbp_gm (Utilities|Casting|CastToBP_GM (Game|GetGameMode)))
  (Variables|Default|SetGMRef _asbp_gm))

(event EventTick
  (params (DeltaSeconds :type Float%20%28single-precision%29)))

(event Input|KeyboardEvents|SpaceBar
  (params (Key :type Key%20Structure))
  (:Pressed
    (bind _asbp_house (Utilities|Casting|CastToBP_House (Variables|Default|GetCurrentActor)))
    (Default|SpawnNewHouse (Variables|Default|GetGMRef) _asbp_house 1e+03 1.5e+03)))

(event Input|MouseEvents|LeftMouseButton
  (params (Key :type Key%20Structure))
  (bind _hitresult (Game|Player|GetHitResultUnderCursorbyChannel "TraceTypeQuery2" true))
  (:Pressed
    (Development|PrintString (Utilities|GetObjectName (.hitactor _hitresult)))
    (if (Utilities|DoesObjectImplementInterface (.hitactor _hitresult) "/Game/Blueprints/Interface/BPI_Interactables.BPI_Interactables_C")
      (Default|Focuson (Variables|Default|GetCamRef) (Transformation|GetActorLocation (.hitactor _hitresult)) 1e+03)
      (bind _output_get (Variables|Default|SetCurrentActor (.hitactor _hitresult)))
      (Class|BPIInteractables|OnClick(Message) _output_get))))

(event Input|KeyboardEvents|1
  (params (Key :type Key%20Structure))
  (:Pressed
    (Class|BPIInteractables|Debug(Message) (Variables|Default|GetCurrentActor) 1)))

(event Input|KeyboardEvents|2
  (params (Key :type Key%20Structure))
  (:Pressed
    (Class|BPIInteractables|Debug(Message) (Variables|Default|GetCurrentActor) 2)))

(event Input|KeyboardEvents|3
  (params (Key :type Key%20Structure))
  (:Pressed
    (Class|BPIInteractables|Debug(Message) (Variables|Default|GetCurrentActor) 3)))

(event Input|KeyboardEvents|4
  (params (Key :type Key%20Structure))
  (:Pressed
    (Class|BPIInteractables|Debug(Message) (Variables|Default|GetCurrentActor) 4)))

(fn ConstructionScript)