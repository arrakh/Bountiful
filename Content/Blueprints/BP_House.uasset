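; BP_House is a clickable house actor that holds a resource inventory and shows it in the HUD when clicked.
; On BeginPlay it caches BP_GM, changes the roof material if it is the home, and starts a looping timer on a still-empty GenerateEvent.
; AddResource increments matching entries or appends new ones from DT_Resource, while RemoveResource subtracts without a floor check.
; A Debug event adds resources as a cheat; RemoveAllResourceNamed is an empty stub.
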(event Custom|GenerateEvent)

(event EventBeginPlay
  (Utilities|FlowControl|Sequence
    (:then_0
      (bind _asbp_gm (Utilities|Casting|CastToBP_GM (Game|GetGameMode)))
      (Variables|Default|SetGMRef _asbp_gm))
    (:then_1
      (if (Variables|Default|GetisHome)
        (Rendering|Material|SetMaterial (Variables|Default|GetRoof) 0 "/Engine/EngineDebugMaterials/MAT_LevelColorationLitLightmapUV.MAT_LevelColorationLitLightmapUV")))
    (:then_2
      (Utilities|Time|SetTimerbyEvent (delegate Custom|GenerateEvent) 1.0 true))))

(event Collision|EventActorBeginOverlap
  (params (OtherActor :type Actor%20Object%20Reference)))

(event EventTick
  (params (DeltaSeconds :type Float%20%28single-precision%29)))

(event EventOnClick
  (Default|InitResourceList (Variables|/Game/Blueprints/Game/BP_GM.BP_GM_C|GetHUDRef (Variables|Default|GetGMRef)) (Variables|Default|GetResourceInventory)))

(event EventDebug
  (params (DebugCode :type Integer))
  (CallFunction|AddResource DebugCode 1)
  (Development|PrintString "CHEAT"))

(fn ConstructionScript)

(fn AddResource
  (params (ItemID :type Integer) (Quantity :type Integer))
  (bind _resourceinventory (Variables|Default|GetResourceInventory))
  (bind _output_get (LocalVariables|SetLocalItemID ItemID))
  (LocalVariables|SetLocalQuan Quantity)
  (bind (_array_element _array_index) (Utilities|Array|ForEachLoopwithBreak (Variables|Default|GetResourceInventory) :!label _label)
    (:LoopBody
      (LocalVariables|SetLocalIndex _array_index)
      (if (== _output_get (.ResourceID (Utilities|Struct|BreakS_ItemData (.itemdata _array_element))))
        (LocalVariables|SetItemFound true)
        (goto _label Break)
        (else
          (LocalVariables|SetItemFound false))))
    (:Completed
      (if (LocalVariables|GetItemFound)
        (Utilities|Array|SetArrayElem _resourceinventory (LocalVariables|GetLocalIndex) (Utilities|Struct|MakeS_ResInventory (.itemdata (Utilities|Array|Get(acopy) _resourceinventory (LocalVariables|GetLocalIndex))) (+ (.quantity (Utilities|Array|Get(acopy) _resourceinventory (LocalVariables|GetLocalIndex))) (LocalVariables|GetLocalQuan)) (.generatepersecond (Utilities|Array|Get(acopy) _resourceinventory (LocalVariables|GetLocalIndex))) (.isgenerate (Utilities|Array|Get(acopy) _resourceinventory (LocalVariables|GetLocalIndex)))))
        (else
          (bind _returnvalue (Utilities|GetDataTableRow "/Game/Data/DT_Resource.DT_Resource" (Utilities|String|StringToName (Utilities|String|ToString(Integer) (LocalVariables|GetLocalItemID))))
            (:then
              (Utilities|Array|Add (Variables|Default|GetResourceInventory) (Utilities|Struct|MakeS_ResInventory _returnvalue (LocalVariables|GetLocalQuan) 0 false)))))))))

(fn RemoveResource
  (params (ItemID :type Integer) (Quantity :type Integer))
  (LocalVariables|SetLocalQuan Quantity)
  (for (_array_element _array_index) (Variables|Default|GetResourceInventory)
    (if (== ItemID (.ResourceID (Utilities|Struct|BreakS_ItemData (.itemdata _array_element))))
      (Utilities|Array|SetArrayElem (Variables|Default|GetResourceInventory) _array_index (Utilities|Struct|MakeS_ResInventory (.itemdata _array_element) (- (.quantity _array_element) (LocalVariables|GetLocalQuan)) (.generatepersecond _array_element) (.isgenerate _array_element))))))

(fn RemoveAllResourceNamed)